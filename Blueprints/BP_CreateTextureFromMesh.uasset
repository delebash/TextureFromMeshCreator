(event EventBeginPlay)

(event Collision|EventActorBeginOverlap
  (params (OtherActor :type Actor%20Object%20Reference)))

(event EventTick
  (params (DeltaSeconds :type Float%20%28single-precision%29)))

(fn ConstructionScript
  (Rendering|SceneCapture|ShowOnlyComponent (Variables|Default|GetSceneCaptureComponent2D_Left) (Variables|Default|GetDynamicMesh_Right))
  (Rendering|SceneCapture|ShowOnlyComponent (Variables|Default|GetSceneCaptureComponent2D_Right) (Variables|Default|GetDynamicMesh_Left)))

(fn PreviewMesh
  (if (Variables|TextureCreator|GetisSkeletalMesh)
    (Variables|TextureCreator|GetSkeletal%20Mesh
      (:then
        (bind _returnvalue (DynamicMeshComponent|GetDynamicMesh (Variables|Default|GetDynamicMesh)))
        (bind _returnvalue_2 (GeometryScript|SkeletalMesh|CopyMeshfromSkeletalMesh (Variables|TextureCreator|GetSkeletal%20Mesh) _returnvalue (Utilities|Struct|MakeGeometryScriptCopyMeshfromAssetOptions true true true) (Utilities|Struct|MakeGeometryScriptMeshReadLOD "MaxAvailable" 0) 0)
          (:Success
            (bind _returnvalue_3 (Class|GeometryScriptLibraryMeshBooleanFunctions|ApplyMeshPlaneCut _returnvalue_2 (Math|Transform|MakeTransform (Variables|TextureCreator|GetCut%20Frame%20Location) "0, 0, 0" "1.000000,1.000000,1.000000") (Utilities|Struct|MakeGeometryScriptMeshPlaneCutOptions false false false 1.0) 0))
            (Variables|TextureCreator|SetDynamic%20Cut%20Mesh _returnvalue_3)
            (for (_array_element _array_index) (Variables|/Script/Engine.SkeletalMesh|GetMaterials (Variables|TextureCreator|GetSkeletal%20Mesh))
              (Rendering|Material|SetMaterial (Variables|Default|GetDynamicMesh_Left) _array_index (.MaterialInterface (Utilities|Struct|BreakSkeletalMaterial _array_element)))
              (Class|DynamicMeshComponent|SetDynamicMesh (Variables|Default|GetDynamicMesh_Left) (Variables|TextureCreator|GetDynamic%20Cut%20Mesh))))))
      (:else))
    (else
      (Variables|TextureCreator|GetStaticMesh
        (:then
          (bind _returnvalue_4 (DynamicMeshComponent|GetDynamicMesh (Variables|Default|GetDynamicMesh)))
          (bind _returnvalue_5 (GeometryScript|StaticMesh|CopyMeshFromStaticMesh :FromStaticMeshAsset (Variables|TextureCreator|GetStaticMesh) :ToDynamicMesh _returnvalue_4 :Debug 0)
            (:Success
              (bind _returnvalue_6 (Class|GeometryScriptLibraryMeshBooleanFunctions|ApplyMeshPlaneCut _returnvalue_5 (Math|Transform|MakeTransform (Variables|TextureCreator|GetCut%20Frame%20Location) "0, 0, 0" "1.000000,1.000000,1.000000") (Utilities|Struct|MakeGeometryScriptMeshPlaneCutOptions false false false 1.0) 0))
              (Variables|TextureCreator|SetDynamic%20Cut%20Mesh _returnvalue_6)
              (for (_array_element_2 _array_index_2) (Variables|/Script/Engine.StaticMesh|GetStaticMaterials (Variables|TextureCreator|GetStaticMesh))
                (Rendering|Material|SetMaterial (Variables|Default|GetDynamicMesh_Left) _array_index_2 (.MaterialInterface (Utilities|Struct|BreakStaticMaterial _array_element_2)))
                (Class|DynamicMeshComponent|SetDynamicMesh (Variables|Default|GetDynamicMesh_Left) (Variables|TextureCreator|GetDynamic%20Cut%20Mesh))))))
        (:else)))))

(fn CreateTexture
  (if (Variables|TextureCreator|GetisSkeletalMesh)
    (Variables|TextureCreator|SetMeshName (Utilities|GetDisplayName (Variables|TextureCreator|GetSkeletal%20Mesh)))
    (else
      (Variables|TextureCreator|SetMeshName (Utilities|GetDisplayName (Variables|TextureCreator|GetStaticMesh)))))
  (Class|KismetRenderingLibrary|RenderTargetCreateStaticTexture2DEditorOnly "/Game/TextureFromMeshCreator/RenderTargets/RT_SceneCapture_Right.RT_SceneCapture_Right" (Utilities|String|Append (Utilities|String|Append (Variables|TextureCreator|GetOutTextureFolder) (Utilities|String|Append "T_" (Variables|TextureCreator|GetMeshName))) "_Right") "TC_HDR_F32" "TMGS_FromTextureGroup")
  (Class|KismetRenderingLibrary|RenderTargetCreateStaticTexture2DEditorOnly "/Game/TextureFromMeshCreator/RenderTargets/RT_SceneCapture_Left.RT_SceneCapture_Left" (Utilities|String|Append (Utilities|String|Append (Variables|TextureCreator|GetOutTextureFolder) (Utilities|String|Append "T_" (Variables|TextureCreator|GetMeshName))) "_Left") "TC_HDR_F32" "TMGS_FromTextureGroup"))

(fn CreateAlpha
  (Rendering|ClearRenderTarget2D "/Game/TextureFromMeshCreator/RenderTargets/RT_Alpha_Left.RT_Alpha_Left")
  (Rendering|ClearRenderTarget2D "/Game/TextureFromMeshCreator/RenderTargets/RT_Alpha_Right.RT_Alpha_Right")
  (Rendering|DrawMaterialtoRenderTarget "/Game/TextureFromMeshCreator/RenderTargets/RT_Alpha_Left.RT_Alpha_Left" "/Game/TextureFromMeshCreator/Material_Instances/MI_Alpha_Left.MI_Alpha_Left")
  (Rendering|DrawMaterialtoRenderTarget "/Game/TextureFromMeshCreator/RenderTargets/RT_Alpha_Right.RT_Alpha_Right" "/Game/TextureFromMeshCreator/Material_Instances/MI_Alpha_Right.MI_Alpha_Right")
  (if (Variables|TextureCreator|GetisSkeletalMesh)
    (Variables|TextureCreator|SetMeshName (Utilities|GetDisplayName (Variables|TextureCreator|GetSkeletal%20Mesh)))
    (else
      (Variables|TextureCreator|SetMeshName (Utilities|GetDisplayName (Variables|TextureCreator|GetStaticMesh)))))
  (Class|KismetRenderingLibrary|RenderTargetCreateStaticTexture2DEditorOnly "/Game/TextureFromMeshCreator/RenderTargets/RT_Alpha_Right.RT_Alpha_Right" (Utilities|String|Append (Utilities|String|Append (Variables|TextureCreator|GetOutTextureFolder) (Utilities|String|Append "T_" (Variables|TextureCreator|GetMeshName))) "_Alpha_Right") "TC_HDR_F32" "TMGS_FromTextureGroup")
  (Class|KismetRenderingLibrary|RenderTargetCreateStaticTexture2DEditorOnly "/Game/TextureFromMeshCreator/RenderTargets/RT_Alpha_Left.RT_Alpha_Left" (Utilities|String|Append (Utilities|String|Append (Variables|TextureCreator|GetOutTextureFolder) (Utilities|String|Append "T_" (Variables|TextureCreator|GetMeshName))) "_Alpha_Left") "TC_HDR_F32" "TMGS_FromTextureGroup"))