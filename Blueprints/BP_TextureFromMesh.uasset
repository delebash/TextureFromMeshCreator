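; Editor tool Blueprint that turns a skeletal or static mesh into left and right foot textures.
; PreviewMesh copies the chosen mesh into a dynamic mesh with Geometry Script, plane-cuts it without filling holes, and writes it to a temporary static mesh with original or white override materials.
; CreateTexture saves the left and right screen-capture render targets as HDR texture assets named after the source mesh.
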(event EventBeginPlay)

(event Collision|EventActorBeginOverlap
  (params (OtherActor :type Actor%20Object%20Reference)))

(event EventTick
  (params (DeltaSeconds :type Float%20%28single-precision%29)))

(fn ConstructionScript)

(fn PreviewMesh
  (if (Variables|CreateTexture|GetisSkeletalMesh)
    (Variables|CreateTexture|GetSkeletal%20Mesh
      (:then
        (Development|PrintString "Hello")
        (bind _returnvalue (DynamicMeshComponent|GetDynamicMesh (Variables|DynamicMeshActor|GetDynamicMeshComponent)))
        (bind _returnvalue_2 (GeometryScript|SkeletalMesh|CopyMeshfromSkeletalMesh (Variables|CreateTexture|GetSkeletal%20Mesh) _returnvalue (Utilities|Struct|MakeGeometryScriptCopyMeshfromAssetOptions true true true) (Utilities|Struct|MakeGeometryScriptMeshReadLOD "MaxAvailable" 0) 0)
          (:Success
            (bind _returnvalue_3 (Class|GeometryScriptLibraryMeshBooleanFunctions|ApplyMeshPlaneCut _returnvalue_2 (Math|Transform|MakeTransform (Variables|CreateTexture|GetCut%20Frame%20Location) "0, 0, 0" "1.000000,1.000000,1.000000") (Utilities|Struct|MakeGeometryScriptMeshPlaneCutOptions false false false 1.0) 0))
            (GeometryScript|StaticMesh|CopyMeshtoStaticMesh :FromDynamicMesh _returnvalue_3 :ToStaticMeshAsset (Variables|CreateTexture|GetTemp%20Static%20Mesh%20Asset) :Debug 0
              (:Success
                (for (_array_element _array_index) (Variables|/Script/Engine.SkeletalMesh|GetMaterials (Variables|CreateTexture|GetSkeletal%20Mesh))
                  (Variables|CreateTexture|SetMaterial%20Index _array_index)
                  (if (Variables|CreateTexture|GetuseWhiteTexture)
                    (Rendering|Material|SetMaterial (Variables|CreateTexture|GetTemp%20Static%20Mesh%20Asset) (Variables|CreateTexture|GetMaterial%20Index) "/Game/TextureFromMeshCreator/Materials/M_Temp_Mesh.M_Temp_Mesh")
                    (else
                      (Rendering|Material|SetMaterial (Variables|CreateTexture|GetTemp%20Static%20Mesh%20Asset) (Variables|CreateTexture|GetMaterial%20Index) (.MaterialInterface (Utilities|Struct|BreakSkeletalMaterial _array_element)))))))))))
      (:else
        (Development|PrintString "not")))
    (else
      (Variables|CreateTexture|GetStaticMesh
        (:then
          (bind _returnvalue_4 (DynamicMeshComponent|GetDynamicMesh (Variables|DynamicMeshActor|GetDynamicMeshComponent)))
          (bind _returnvalue_5 (GeometryScript|StaticMesh|CopyMeshFromStaticMesh :FromStaticMeshAsset (Variables|CreateTexture|GetStaticMesh) :ToDynamicMesh _returnvalue_4 :Debug 0)
            (:Success
              (bind _returnvalue_6 (Class|GeometryScriptLibraryMeshBooleanFunctions|ApplyMeshPlaneCut _returnvalue_5 (Math|Transform|MakeTransform (Variables|CreateTexture|GetCut%20Frame%20Location) "0, 0, 0" "1.000000,1.000000,1.000000") (Utilities|Struct|MakeGeometryScriptMeshPlaneCutOptions false false false 1.0) 0))
              (GeometryScript|StaticMesh|CopyMeshtoStaticMesh :FromDynamicMesh _returnvalue_6 :ToStaticMeshAsset (Variables|CreateTexture|GetTemp%20Static%20Mesh%20Asset) :Debug 0
                (:Success
                  (for (_array_element_2 _array_index_2) (Variables|/Script/Engine.StaticMesh|GetStaticMaterials (Variables|CreateTexture|GetStaticMesh))
                    (Variables|CreateTexture|SetMaterial%20Index _array_index_2)
                    (if (Variables|CreateTexture|GetuseWhiteTexture)
                      (Rendering|Material|SetMaterial (Variables|CreateTexture|GetTemp%20Static%20Mesh%20Asset) (Variables|CreateTexture|GetMaterial%20Index) "/Game/TextureFromMeshCreator/Materials/M_Temp_Mesh.M_Temp_Mesh")
                      (else
                        (Rendering|Material|SetMaterial (Variables|CreateTexture|GetTemp%20Static%20Mesh%20Asset) (Variables|CreateTexture|GetMaterial%20Index) (.MaterialInterface (Utilities|Struct|BreakStaticMaterial _array_element_2)))))))))))
        (:else)))))

(fn CreateTexture
  (if (Variables|CreateTexture|GetisSkeletalMesh)
    (Variables|CreateTexture|SetMeshName (Utilities|GetDisplayName (Variables|CreateTexture|GetSkeletal%20Mesh)))
    (else
      (Variables|CreateTexture|SetMeshName (Utilities|GetDisplayName (Variables|CreateTexture|GetStaticMesh)))))
  (Class|KismetRenderingLibrary|RenderTargetCreateStaticTexture2DEditorOnly "/Game/TextureFromMeshCreator/RenderTargets/RT_ScreenCapture_Right.RT_ScreenCapture_Right" (Utilities|String|Append (Utilities|String|Append (Variables|CreateTexture|GetOutTextureFolder) (Variables|CreateTexture|GetMeshName)) "_Right_Foot") "TC_HDR_F32" "TMGS_FromTextureGroup")
  (Class|KismetRenderingLibrary|RenderTargetCreateStaticTexture2DEditorOnly "/Game/TextureFromMeshCreator/RenderTargets/RT_ScreenCapture_Left.RT_ScreenCapture_Left" (Utilities|String|Append (Utilities|String|Append (Variables|CreateTexture|GetOutTextureFolder) (Variables|CreateTexture|GetMeshName)) "_Left_Foot") "TC_HDR_F32" "TMGS_FromTextureGroup"))